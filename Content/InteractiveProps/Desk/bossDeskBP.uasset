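; Interactive boss desk prop that plays animations for its intact, wobbling and broken-open states.
; BeginPlay sets the pre-break animation, and separate events trigger the wobble or break-open animation, both with the same safe-opening sound at the desk's location.
; SetFutureSelf plays the post-open animation without sound, putting the desk in its already-opened state.
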(event Custom|DoDeskWobble
  (bind _bossdesk (Variables|Default|GetBossDesk))
  (Components|Animation|PlayAnimation _bossdesk "/Game/InteractiveProps/Desk/BossDesk_Anim_Desk_Wobble.BossDesk_Anim_Desk_Wobble" false)
  (Audio|PlaySoundatLocation "/Game/Assets/Sound/Safe_Opening_Matched.Safe_Opening_Matched" (Transformation|GetWorldLocation _bossdesk) "0, 0, 0" 1.0 1.0 0.0 0 0 0))

(event Custom|DoDeskOpen
  (bind _bossdesk (Variables|Default|GetBossDesk))
  (Components|Animation|PlayAnimation _bossdesk "/Game/InteractiveProps/Desk/BossDesk_Anim_Desk_BreakOpen.BossDesk_Anim_Desk_BreakOpen" false)
  (Audio|PlaySoundatLocation "/Game/Assets/Sound/Safe_Opening_Matched.Safe_Opening_Matched" (Transformation|GetWorldLocation _bossdesk) "0, 0, 0" 1.0 1.0 0.0 0 0 0))

(event Custom|SetFutureSelf
  (Components|Animation|PlayAnimation (Variables|Default|GetBossDesk) "/Game/InteractiveProps/Desk/BossDesk_Anim_Desk_Pst_Open.BossDesk_Anim_Desk_Pst_Open" false))

(event EventBeginPlay
  (Components|Animation|PlayAnimation (Variables|Default|GetBossDesk) "/Game/InteractiveProps/Desk/BossDesk_Anim_Desk_Pre.BossDesk_Anim_Desk_Pre" false))

(fn ConstructionScript)